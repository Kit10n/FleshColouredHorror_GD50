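; HorrorGameMode is the game mode for a horror game, reloading the current level when the player character is destroyed.
; On BeginPlay, CheckCurse uses the real system clock: after 21:30, a random roll against PercentChance schedules a delayed Curse.
; Curse capsule-traces behind the player, spawning a HorrorCharacterZombie there facing them if clear.
; If the trace is blocked, it retries on a one-second timer.
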(event `self.ReceiveBeginPlay`
  (`self.CheckCurse`)
  ;[1 1 1] Reload level when character is destroyed
  (add `self.OnDestroyed` (`GameplayStatics.GetPlayerCharacter` 0) (delegate `CharacterDestroyed`)))

(event `CharacterDestroyed` :!signature `self.OnDestroyed`
  (params (DestroyedActor :type "Actor Object Reference"))
  ;[1 1 1] Reload level when character is destroyed
  (bind _returnvalue (`GameplayStatics.GetCurrentLevelName` true))
  (`GameplayStatics.OpenLevel` (`KismetStringLibrary.Conv_StringToName` _returnvalue)))

(fn `CheckCurse`
  (locals (PercentChance :type "Float (double-precision)" :default 0.04))
  ;[1 1 1] Comment
  (if (> (`KismetMathLibrary.GetTimeOfDay` (`KismetMathLibrary.Now`)) (`KismetMathLibrary.MakeTimespan` 0 21 30))
    ;[1 1 1] Comment
    (`/Engine/EditorBlueprintResources/StandardMacros.CompareFloat` (`KismetMathLibrary.RandomFloat`) (`local.PercentChance`)
      (:`==`
        _)
      (:`<`
        _))
    ;[1 1 1] Comment
    (`KismetSystemLibrary.K2_SetTimer` null "Curse" 2.0)))

(fn `Curse`
  (bind _returnvalue (`GameplayStatics.GetPlayerCharacter` 0))
  (bind _returnvalue_2 (+ (* (`self.GetActorForwardVector` _returnvalue) -200.0) (`self.K2_GetActorLocation` _returnvalue)))
  (bind (_outhit _returnvalue_3) (`KismetSystemLibrary.CapsuleTraceSingle` (`self.K2_GetActorLocation` (`GameplayStatics.GetPlayerCharacter` 0)) _returnvalue_2 30.0 90.0 "TraceTypeQuery1" false (`|MakeArray` (`GameplayStatics.GetPlayerCharacter` 0) :!type "Actor Object Reference")))
  (if (not _returnvalue_3)
    (`AIBlueprintHelperLibrary.SpawnAIFromClass` "/Game/Blueprints/Character/HorrorCharacterZombie.HorrorCharacterZombie_C" null _returnvalue_2 (`KismetMathLibrary.FindLookAtRotation` _returnvalue_2 (`self.K2_GetActorLocation` (`GameplayStatics.GetPlayerCharacter` 0))) true)
    (else
      (`KismetSystemLibrary.K2_SetTimer` null "Curse" 1.0))))

(fn `UserConstructionScript`)