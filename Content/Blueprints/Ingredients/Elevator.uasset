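; An interactable elevator for a first-person horror game that alternates between rising 600 units and returning on each interaction.
; Overlapping the trigger as the player character shows instruction text and opens a Gate that allows interaction; ending overlap hides and closes it.
; A FlipFlop plays or reverses a Timeline that lerps the owning actor's location from the floor's initial position.
; Start, delayed loop and stop sounds accompany the movement.
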(event `self.ReceiveBeginPlay`
  (set `self.v_ElevatorLocation` (`SceneComponent.K2_GetComponentLocation` (`self.ElevatorFloor`))))

(event `/Game/Blueprints/Ingredients/BP_Interact.OnInteract`
  (bind _v_elevatorlocation (`self.v_ElevatorLocation`))
  (`/Engine/EditorBlueprintResources/StandardMacros.Gate` true :!label _label
    (:`Exit`
      (`GameplayStatics.PlaySound2D` "/Game/Audio/SFX/SFX_ElevatorStart.SFX_ElevatorStart") ; elevator start sound
      (`|ExecutionSequence`
        (:`then_0`
          (`/Engine/EditorBlueprintResources/StandardMacros.FlipFlop` ; Elevator up and down
            (:`A`
              (bind (_direction _movement) (`Timeline|Elevator movement` :!label _label_2)
                (:`Update`
                  (`self.K2_SetActorLocation` (`ActorComponent.GetOwner` (`self.ElevatorFloor`)) (`KismetMathLibrary.VLerp` _v_elevatorlocation (+ _v_elevatorlocation (0.0 0.0 600.0)) _movement) false false))
                (:`Finished`
                  (`GameplayStatics.PlaySound2D` "/Game/Audio/SFX/SFX_ElevatorStop.SFX_ElevatorStop") ; Elevator stop sound
                  (`AudioComponent.Stop` (`self.v_loopingSound`)) ; Stop looping elevator sound
                )))
            (:`B`
              (goto _label_2 :!via `Reverse`))))
        (:`then_1`
          (`KismetSystemLibrary.Delay` 0.4) ; Delay loop sound
          (bind _returnvalue (`GameplayStatics.SpawnSoundAtLocation` "/Game/Audio/SFX/SFX_ElevatorLoop.SFX_ElevatorLoop" (0.0 0.0 600.0))) ; Elevator loop sound
          (set `self.v_loopingSound` _returnvalue) ; Variable for looping sound
        )))))

(event `self.ElevatorTrigger.OnComponentBeginOverlap`
  (params (OverlappedComponent :type "PrimitiveComponent Object Reference") (OtherActor :type "Actor Object Reference") (OtherComp :type "PrimitiveComponent Object Reference") (OtherBodyIndex :type Integer) (bFromSweep :type Boolean) (SweepResult :type "HitResult Structure (by ref)"))
  (cast `/Game/Blueprints/Character/HorrorFirstPersonCharacter` OtherActor)
  (`SceneComponent.SetVisibility` (`self.ElevatorInstruction`) true false) ; Change visibility of text actor
  (goto _label :!via `Open`))

(event `self.ReceiveActorEndOverlap`
  (params (OtherActor :type "Actor Object Reference"))
  (cast `/Game/Blueprints/Character/HorrorFirstPersonCharacter` OtherActor)
  (`SceneComponent.SetVisibility` (`self.ElevatorInstruction`) false false) ; Stop changeing visibility
  (goto _label :!via `Close`))

(fn `UserConstructionScript`)