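; BP_Medic is an interactable Blueprint that, despite its name, behaves as a lockable door.
; An interface OnInteract event calls OpenDoor, which checks IsLocked and plays animations on DoorSkeletalMesh.
; When unlocked, a DoOnce gate plays the open animation a single time, with no close or reset logic; when locked, each attempt plays a handle shake.
; SetDoorLocked sets the lock state.
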(event `/Game/Blueprints/Ingredients/BP_Interact.OnInteract`
  ;[1 1 1] Interface
  (`self.OpenDoor`))

(event `OpenDoor`
  ;[1 1 1] Open/Close Door
  (if (not (`self.IsLocked`))
    (`/Engine/EditorBlueprintResources/StandardMacros.DoOnce` false
      (:`Completed`
        (`SkeletalMeshComponent.PlayAnimation` (`self.DoorSkeletalMesh`) "/Game/Environment/Animation/Anim_Door_CompositeOpen.Anim_Door_CompositeOpen" false)))
    (else
      (`SkeletalMeshComponent.PlayAnimation` (`self.DoorSkeletalMesh`) "/Game/Environment/Animation/Anim_Door_HandleShake.Anim_Door_HandleShake" false))))

(fn `SetDoorLocked`
  (params (IsLocked :type Boolean))
  (set `self.IsLocked` IsLocked))

(fn `UserConstructionScript`)