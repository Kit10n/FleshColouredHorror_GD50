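; VanishDoctor is a one-shot horror scare that makes a doctor figure vanish when the player enters its trigger.
; The Activation overlap hides the Doctor, disables player input and plays a breathing sound.
; After a short delay, it destroys its root, doctor and trigger components, swaps the referenced TV's material to look switched on, restores input and starts the TV sound.
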(event `self.Activation.OnComponentBeginOverlap`
  (params (OverlappedComponent :type "PrimitiveComponent Object Reference") (OtherActor :type "Actor Object Reference") (OtherComp :type "PrimitiveComponent Object Reference") (OtherBodyIndex :type Integer) (bFromSweep :type Boolean) (SweepResult :type "HitResult Structure (by ref)"))
  (bind _returnvalue (`GameplayStatics.GetPlayerPawn` 0))
  ;[1 1 1] Vanshing doctor
  (cast `/Game/Blueprints/Character/HorrorFirstPersonCharacter` OtherActor)
  (`/Engine/EditorBlueprintResources/StandardMacros.DoOnce` false
    (:`Completed`
      (`SceneComponent.ToggleVisibility` (`self.Doctor`) false) ; Make doctor vanish
      (`self.DisableInput` _returnvalue null) ; disable controls
      (`GameplayStatics.SpawnSound2D` "/Game/Audio/SFX/SFX_PlayerBreathing_Cue.SFX_PlayerBreathing_Cue") ; Play sound of player
      (`KismetSystemLibrary.Delay` 1.3)
      (`ActorComponent.K2_DestroyComponent` (`self.DefaultSceneRoot`))
      (`ActorComponent.K2_DestroyComponent` (`self.Doctor`))
      (`ActorComponent.K2_DestroyComponent` (`self.Activation`)) ; Destroy doctor
      (`PrimitiveComponent.SetMaterial` (`/Game/Blueprints/Ingredients/TVGuyON.TV` (`self.R_TVRef`)) 0 "/Game/Props/Materials/MI_LampLight_01.MI_LampLight_01") ; Change material of TV to turn it "on"
      (`ActorComponent.ToggleActive` (`self.TVSound`)) ; Turn on audio component
      (`|ExecutionSequence`
        (:`then_0`
          (`self.EnableInput` _returnvalue null) ; Enable controls
        )
        (:`then_1`
          (`AudioComponent.Play` (`self.TVSound`) 0.0) ; play sound
        )))))

(fn `UserConstructionScript`)