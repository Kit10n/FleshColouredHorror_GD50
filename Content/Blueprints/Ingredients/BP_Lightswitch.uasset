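; BP_Lightswitch is an interactable light switch that turns a spotlight on and off.
; OnInteract calls Interaction, which branches on VLightOn to LightOn or LightOff, both updating the flag and toggling SpotLight visibility.
; Trigger begin and end overlaps share a FlipFlop path that toggles TextRender visibility, without filtering the overlapping actor.
; Visibility is toggled rather than set, so it depends on each component's starting state.
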(event `/Game/Blueprints/Ingredients/BP_Interact.OnInteract`
  (`self.Interaction`))

(event `Light On`
  (set `self.V_Light_On` true)
  (`SceneComponent.ToggleVisibility` (`self.SpotLight`) false :!label _label))

(event `Interaction`
  (if (`self.V_Light_On`)
    (`self.Light Off`)
    (else
      (`self.Light On`))))

(event `Light Off`
  (set `self.V_Light_On` false)
  (goto _label))

(event `self.trigger.OnComponentBeginOverlap`
  (params (OverlappedComponent :type "PrimitiveComponent Object Reference") (OtherActor :type "Actor Object Reference") (OtherComp :type "PrimitiveComponent Object Reference") (OtherBodyIndex :type Integer) (bFromSweep :type Boolean) (SweepResult :type "HitResult Structure (by ref)"))
  (bind _isa (`/Engine/EditorBlueprintResources/StandardMacros.FlipFlop` :!label _label_2)
    (:`A`
      _)
    (:`B`
      _))
  (`SceneComponent.ToggleVisibility` (`self.TextRender`) _isa))

(event `self.trigger.OnComponentEndOverlap`
  (params (OverlappedComponent :type "PrimitiveComponent Object Reference") (OtherActor :type "Actor Object Reference") (OtherComp :type "PrimitiveComponent Object Reference") (OtherBodyIndex :type Integer))
  (goto _label_2))

(fn `UserConstructionScript`)