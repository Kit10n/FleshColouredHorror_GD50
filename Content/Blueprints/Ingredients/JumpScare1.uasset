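; JumpScare1 is a one-shot zombie jump scare triggered when the HorrorFirstPersonCharacter overlaps its Activation component.
; It toggles the ZombieAttack mesh's visibility and active state, disables player input and turns the view toward the actor's root with a single RInterpTo call.
; An attack animation and a 2D death sound play, then delays time the destruction of its components and the return of input.
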(event `self.Activation.OnComponentBeginOverlap`
  (params (OverlappedComponent :type "PrimitiveComponent Object Reference") (OtherActor :type "Actor Object Reference") (OtherComp :type "PrimitiveComponent Object Reference") (OtherBodyIndex :type Integer) (bFromSweep :type Boolean) (SweepResult :type "HitResult Structure (by ref)"))
  (bind _returnvalue (`GameplayStatics.GetPlayerPawn` 0))
  (bind _returnvalue_2 (`GameplayStatics.GetPlayerController` 0))
  ;[1 1 1] Jump scare
  (cast `/Game/Blueprints/Character/HorrorFirstPersonCharacter` OtherActor)
  (`SceneComponent.ToggleVisibility` (`self.Zombie attack`) false)
  (`ActorComponent.ToggleActive` (`self.Zombie attack`))
  (`self.DisableInput` _returnvalue null)
  (`Controller.SetControlRotation` _returnvalue_2 (`KismetMathLibrary.RInterpTo` (`Controller.GetControlRotation` _returnvalue_2) (`KismetMathLibrary.FindLookAtRotation` (`self.K2_GetActorLocation` _returnvalue) (`SceneComponent.K2_GetComponentLocation` (`self.DefaultSceneRoot`))) (`GameplayStatics.GetWorldDeltaSeconds`)))
  (`SkeletalMeshComponent.PlayAnimation` (`self.Zombie attack`) "/Game/Characters/Zombie/Animations/Anim_Zombie01_Attack02.Anim_Zombie01_Attack02" false)
  (`GameplayStatics.SpawnSound2D` "/Game/Audio/SFX/SFX_PlayerDeathShort01.SFX_PlayerDeathShort01")
  (`KismetSystemLibrary.Delay` 1.7)
  (`ActorComponent.K2_DestroyComponent` (`self.DefaultSceneRoot`))
  (`ActorComponent.K2_DestroyComponent` (`self.Zombie attack`))
  (`ActorComponent.K2_DestroyComponent` (`self.Activation`))
  (`KismetSystemLibrary.Delay` 1.8)
  (`self.EnableInput` _returnvalue null))

(fn `UserConstructionScript`)