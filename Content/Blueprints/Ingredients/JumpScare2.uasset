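; Jump scare actor that fires when the horror first-person character overlaps its Activation component.
; It toggles the zombie mesh's visibility and active state, disables input, turns the view toward its root, then plays an animation and 2D death sound.
; After a short delay it destroys its root, zombie and trigger components, then restores input after another delay.
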(event `self.Activation.OnComponentBeginOverlap`
  (params (OverlappedComponent :type "PrimitiveComponent Object Reference") (OtherActor :type "Actor Object Reference") (OtherComp :type "PrimitiveComponent Object Reference") (OtherBodyIndex :type Integer) (bFromSweep :type Boolean) (SweepResult :type "HitResult Structure (by ref)"))
  (bind _returnvalue (`GameplayStatics.GetPlayerController` 0))
  ;[1 1 1] Jump scare
  (cast `/Game/Blueprints/Character/HorrorFirstPersonCharacter` OtherActor)
  (`SceneComponent.ToggleVisibility` (`self.Zombie attack`) false)
  (`ActorComponent.ToggleActive` (`self.Zombie attack`))
  (`self.DisableInput` _returnvalue null)
  (`Controller.SetControlRotation` _returnvalue (`KismetMathLibrary.RInterpTo` (`Controller.GetControlRotation` _returnvalue) (`KismetMathLibrary.FindLookAtRotation` (`self.K2_GetActorLocation` _returnvalue) (`SceneComponent.K2_GetComponentLocation` (`self.DefaultSceneRoot`))) (`GameplayStatics.GetWorldDeltaSeconds`)))
  (`SkeletalMeshComponent.PlayAnimation` (`self.Zombie attack`) "/Game/Characters/Doctor/Anims/Anim_Doctor_Idle.Anim_Doctor_Idle" false)
  (`GameplayStatics.SpawnSound2D` "/Game/Audio/SFX/SFX_PlayerDeathShort_Cue.SFX_PlayerDeathShort_Cue")
  (`KismetSystemLibrary.Delay` 1.7)
  (`ActorComponent.K2_DestroyComponent` (`self.DefaultSceneRoot`))
  (`ActorComponent.K2_DestroyComponent` (`self.Zombie attack`))
  (`ActorComponent.K2_DestroyComponent` (`self.Activation`))
  (`KismetSystemLibrary.Delay` 2.0)
  (`self.EnableInput` _returnvalue null))

(fn `UserConstructionScript`)