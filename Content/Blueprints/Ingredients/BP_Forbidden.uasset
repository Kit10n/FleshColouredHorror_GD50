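; BP_Forbidden is an interactable embryo ingredient that, when taken, releases an enemy to chase.
; On interact it casts the referenced RCrazyLady to AI_Enemy2, toggles its mesh and movement active states, sets its AI state and toggles mesh visibility.
; A DoOnce then destroys the pickup.
; The enemy is an existing actor reference switched on by toggles, despite the comment describing a spawn.
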(event `/Game/Blueprints/Ingredients/BP_Interact.OnInteract`
  (bind _r_crazylady (`self.R_CrazyLady`))
  ;[1 1 1] Take the embryo and spawn enemies to chase
  (bind _asai_enemy_2 (cast `/Game/Blueprints/AI/AI_Enemy2` _r_crazylady))
  (`ActorComponent.ToggleActive` (`Character.Mesh` _r_crazylady))
  (`ActorComponent.ToggleActive` (`Character.CharacterMovement` _r_crazylady))
  (set `/Game/Blueprints/AI/AI_Enemy2.AI_State` "NewEnumerator3" _asai_enemy_2)
  (`SceneComponent.ToggleVisibility` (`Character.Mesh` _asai_enemy_2) false)
  (`/Engine/EditorBlueprintResources/StandardMacros.DoOnce` false
    (:`Completed`
      (`self.K2_DestroyActor`))))

(fn `UserConstructionScript`)