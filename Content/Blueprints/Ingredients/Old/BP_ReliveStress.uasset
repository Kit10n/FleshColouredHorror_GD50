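; BP_ReliveStress is an interactable potion the player drinks, altering the horror character's heart rate.
; On its first interaction only, it checks that the med door is open and the player's current heart rate is below maximum.
; If so, it adds a fixed, unclamped amount, broadcasts the heart-rate update and destroys itself.
; The DoOnce precedes both checks, so a failed first attempt also uses it up.
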(event `/Game/Blueprints/Ingredients/BP_Interact.OnInteract`
  ;[1 1 1] Drink potion after door is opened
  (`/Engine/EditorBlueprintResources/StandardMacros.DoOnce` false
    (:`Completed`
      (if (`self.V_MedDoorOpen`)
        (bind _ashorror_first_person_character (cast `/Game/Blueprints/Character/HorrorFirstPersonCharacter` (`GameplayStatics.GetPlayerCharacter` 0)))
        (if (< (`/Game/Blueprints/Character/HorrorFirstPersonCharacter.V_Current_HeartRate` _ashorror_first_person_character) (`/Game/Blueprints/Character/HorrorFirstPersonCharacter.V_Max_HeartRate` _ashorror_first_person_character))
          (bind _output_get (set `/Game/Blueprints/Character/HorrorFirstPersonCharacter.V_Current_HeartRate` (+ (`/Game/Blueprints/Character/HorrorFirstPersonCharacter.V_Current_HeartRate` _ashorror_first_person_character) 40.0) _ashorror_first_person_character))
          (`/Game/Blueprints/Character/HorrorFirstPersonCharacter.Update_Heartrate__DelegateSignature` _ashorror_first_person_character _output_get)
          (`self.K2_DestroyActor`))))))

(fn `UserConstructionScript`)