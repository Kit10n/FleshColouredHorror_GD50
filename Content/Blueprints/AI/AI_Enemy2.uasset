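; Horror-game enemy AI that roams random navigable points, patrols target points or chases the player, chosen by an AIState enum.
; PawnSensing sightings start a chase that re-issues AIMoveTo on a delay, falling back to patrol on failure or disabled sensing.
; Reaching the player applies damage with explosion and sound effects.
; The player's death event disables sensing and re-runs the state switch.
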(event `self.ReceiveBeginPlay`
  ;[1 1 1] Switch State of AI with Enumerator. And Reset AI if player died
  (bind _ashorror_first_person_character (cast `/Game/Blueprints/Character/HorrorFirstPersonCharacter` (`GameplayStatics.GetPlayerCharacter` 0)))
  (add `/Game/Blueprints/Character/HorrorFirstPersonCharacter.Player_is_Dead` _ashorror_first_person_character (delegate `Reset AI`))
  (switch `/Game/Blueprints/AI/E_AI_State` (`self.AI_State`) :!label _label
    (:`NewEnumerator1`
      (`self.Roam`))
    (:`NewEnumerator2`
      (`self.Patrol to points`))
    (:`NewEnumerator3`
      (`self.Chase` null))))

(event `Reset AI`
  ;[1 1 1] Switch State of AI with Enumerator. And Reset AI if player died
  (`PawnSensingComponent.SetSensingUpdatesEnabled` (`self.PawnSensing`) false)
  (goto _label))

(event `Roam`
  ;[1 1 1] AI Roam
  (`|AIMoveTo` self (`NavigationSystem.K2_GetRandomLocationInNavigableRadius` (`self.K2_GetActorLocation`) 10000.0)
    (:`OnSuccess`
      (`KismetSystemLibrary.Delay` 3.0)
      (`self.Roam`)
      (switch `/Game/Blueprints/AI/E_AI_State` (`self.AI_State`)
        (:`NewEnumerator1`
          (`self.Roam`))
        (:`NewEnumerator2`
          (`self.Patrol to points`))
        (:`NewEnumerator3`
          (`self.Chase` null))))))

(event `Chase`
  (params (PlayerToChase :type "Pawn Object Reference"))
  (bind _returnvalue (`self.K2_GetActorLocation`))
  ;[1 1 1] AI chase
  (if (`PawnSensingComponent.bEnableSensingUpdates` (`self.PawnSensing`))
    (`|AIMoveTo` self (0.0 0.0 0.0) PlayerToChase
      (:`then`
        (if (`PawnSensingComponent.bEnableSensingUpdates` (`self.PawnSensing`))
          (`KismetSystemLibrary.Delay` 1.0)
          (`self.Chase` PlayerToChase)
          (else
            (`self.Patrol to points` :!label _label_2))))
      (:`OnSuccess`
        (`GameplayStatics.ApplyDamage` PlayerToChase (`self.HeartBeat`))
        (`GameplayStatics.SpawnEmitterAtLocation` "/Game/Effects/Particles/P_Explosion.P_Explosion" _returnvalue)
        (`GameplayStatics.PlaySoundAtLocation` "/Game/Audio/SFX/SFX_Impact14.SFX_Impact14" _returnvalue (struct) 2.0)
        (`GameplayStatics.PlaySoundAtLocation` "/Game/Audio/SFX/SFX_PlayerDeathShort01.SFX_PlayerDeathShort01" (`self.K2_GetActorLocation` (`GameplayStatics.GetPlayerCharacter` 0))))
      (:`OnFail`
        (goto _label_2)))))

(event `Patrol to points`
  ;[1 1 1] AI Patrol
  (`|AIMoveTo` self (0.0 0.0 0.0) (`|GetArrayItem` (`self.TargetPoints`) (`self.PatrolPointIndex`))
    (:`OnSuccess`
      (`KismetSystemLibrary.Delay` 3.0)
      (if (>= (`self.PatrolPointIndex`) (- (`KismetArrayLibrary.Array_Length` (`self.TargetPoints`)) 1))
        (set `self.PatrolPointIndex` 0)
        (else
          (`/Engine/EditorBlueprintResources/StandardMacros.IncrementInt` (`self.PatrolPointIndex`)
            (:`  `
              _))))
      (`self.Patrol to points`))))

(event `self.PawnSensing.OnSeePawn`
  (params (Pawn :type "Pawn Object Reference"))
  ;[1 1 1] Chase player when AI sees player pawn
  (bind _ashorror_first_person_character (cast `/Game/Blueprints/Character/HorrorFirstPersonCharacter` Pawn))
  (`self.Chase` _ashorror_first_person_character)
  (`PawnSensingComponent.SetSensingUpdatesEnabled` (`self.PawnSensing`) true))

(fn `UserConstructionScript`)