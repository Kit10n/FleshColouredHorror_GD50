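; Physics projectile Blueprint that pushes simulated bodies and breaks destructible actors on impact.
; On each collision component hit it stores the actor, component and hit result, then applies an impulse against the impact normal at the impact point if that component simulates physics.
; If the hit actor is a DestructibleActor, it also applies radius damage with an impulse to its destructible component at that point.
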(event `self.ProjectileCollision.OnComponentHit`
  (params (OtherActor :type "Actor Object Reference") (OtherComp :type "PrimitiveComponent Object Reference") (NormalImpulse :type "Vector Structure") (Hit :type "HitResult Structure (by ref)"))
  (bind (_lasthit_bblockinghit _lasthit_binitialoverlap _lasthit_time _lasthit_location _lasthit_impactpoint _lasthit_normal _lasthit_impactnormal) (`GameplayStatics.BreakHitResult` (`self.LastHit`)))
  (bind (_lasthit_bblockinghit_2 _lasthit_binitialoverlap_2 _lasthit_time_2 _lasthit_location_2 _lasthit_impactpoint_2) (`GameplayStatics.BreakHitResult` (`self.LastHit`)))
  ;[1 1 1] Store for later
  (set `self.LastHitActor` OtherActor)
  (set `self.LastHitComponent` OtherComp)
  (set `self.LastHit` Hit)
  ;[1 1 1] For physics actors
  (if (`SceneComponent.IsSimulatingPhysics` (`self.LastHitComponent`) "None")
    (`PrimitiveComponent.AddImpulseAtLocation` (`self.LastHitComponent`) (* (`KismetMathLibrary.NegateVector` _lasthit_impactnormal) 10000.0) _lasthit_impactpoint "None"))
  ;[1 1 1] For destructibles
  (bind _asdestructible_actor (cast `DestructibleActor` (`self.LastHitActor`)))
  (`DestructibleComponent.ApplyRadiusDamage` (`DestructibleActor.DestructibleComponent` _asdestructible_actor) 1.0 _lasthit_impactpoint_2 64.0 10000.0 false))

(fn `UserConstructionScript`)